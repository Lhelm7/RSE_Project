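; Enemy missile pawn that homes in on the player character and triggers a game reset when it reaches them.
; Move activates it and starts AI MoveTo, which on success flags the player dead in the GameInstance.
; CallNextMissile plays explosion and voice cues, destroys the missile and has the GameMode launch the next.
; Tick runs sonar audio while active, switching once to a faster loop when X-axis distance closes.
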(event Custom|Move
  (Variables|Default|SetIsActive true)
  (AI|AIMoveTo self "0, 0, 0" (Variables|Default|GetAs%20BP%20Character) 2e+01 false
    (:OnSuccess
      (Variables|/Game/Game/Blueprints/BP_Gameinstance.BP_Gameinstance_C|SetPlayerDed (Variables|Default|GetAs%20BP%20Gameinstance) true)
      (Actor|DestroyActor)
      (Default|ResetGame (Variables|Default|GetAs%20BP%20Gamemode)))))

(event Custom|CallNextMissile
  (Audio|PlaySoundatLocation "/Game/Game/Sounds/Commencer_Arrêter_RSE/SoundDesign_RSE/SoundExplosion/nuke-333673_Cue.nuke-333673_Cue" (Transformation|GetActorLocation) "0, 0, 0" 0.1 1.0 0.0 0 0 0 0)
  (Audio|PlaySound2D "/Game/Game/Sounds/Commencer_Arrêter_RSE/SoundDesign_RSE/ElevenLabs_Text_to_Speech_audio_Cue.ElevenLabs_Text_to_Speech_audio_Cue" 1.0 1.0 0.0 0 0)
  (Actor|DestroyActor)
  (Default|CallMoveNextMissile (Variables|Default|GetAs%20BP%20Gamemode)))

(event EventBeginPlay
  (bind _asbp_character (Utilities|Casting|CastToBP_Character (Game|Player|GetPlayerPawn 0)))
  (Variables|Default|SetAs%20BP%20Character _asbp_character)
  (bind _asbp_gamemode (Utilities|Casting|CastToBP_Gamemode (Game|GetGameMode)))
  (Variables|Default|SetAs%20BP%20Gamemode _asbp_gamemode)
  (bind _asbp_gameinstance (Utilities|Casting|CastToBP_Gameinstance (Game|GetGameInstance)))
  (Variables|Default|SetAs%20BP%20Gameinstance _asbp_gameinstance))

(event Collision|EventActorBeginOverlap
  (params (OtherActor :type Actor%20Object%20Reference)))

(event EventTick
  (params (DeltaSeconds :type Float%20%28single-precision%29))
  (if (<= (Math|Float|Absolute(Float) (.x (- (Transformation|GetActorLocation (Variables|Default|GetAs%20BP%20Character)) (Transformation|GetActorLocation)))) 1e+03)
    (Utilities|FlowControl|DoOnce false
      (:Completed
        (Audio|Components|Audio|SetSound (Variables|Default|GetSonarAmbiance) "/Game/Game/Sounds/Commencer_Arrêter_RSE/SoundDesign_RSE/SonarAmbianceFast.SonarAmbianceFast"))))
  (if (Variables|Default|GetIsActive)
    (Components|Activation|Activate (Variables|Default|GetSonarAmbiance) false)
    (else
      (Components|Activation|Deactivate (Variables|Default|GetSonarAmbiance)))))

(fn ConstructionScript)