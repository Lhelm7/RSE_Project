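; BP_Gamemode is the game mode that launches enemy missiles one after another.
; On BeginPlay it gathers all BP_MissileEnnemi actors, waits briefly, moves the first and sets it as the player character's focused missile.
; It also binds MoveNext to a MoveNextMissile event, so each call increments an index and moves the corresponding missile in the list, without updating the focused missile.
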(event Custom|MoveNext
  (Development|PrintString "je move le next")
  (bind _result (Math|Integer|IncrementInt (Variables|Default|GetIndex))
    (:%20%20
      (Default|Move (Utilities|Array|Get(acopy) (Variables|Default|GetListOfMissiles) _result)))))

(event EventBeginPlay
  (bind _outactors (Actor|GetAllActorsOfClass "/Game/Game/Blueprints/BP_MissileEnnemi.BP_MissileEnnemi_C"))
  (Variables|Default|SetListOfMissiles _outactors)
  (Utilities|FlowControl|Delay 3.0)
  (Default|Move (Utilities|Array|Get(acopy) (Variables|Default|GetListOfMissiles)))
  (EventDispatchers|BindEventtoMoveNextMissile (delegate Custom|MoveNext))
  (bind _asbp_character (Utilities|Casting|CastToBP_Character (Game|Player|GetPlayerPawn 0)))
  (bind _output_get (Variables|Default|SetAs%20BP%20Character _asbp_character))
  (Variables|/Game/Game/Blueprints/BP_Character.BP_Character_C|SetMissileFocused _output_get (Utilities|Array|Get(acopy) (Variables|Default|GetListOfMissiles))))

(event EventTick
  (params (DeltaSeconds :type Float%20%28single-precision%29)))

(fn ConstructionScript)